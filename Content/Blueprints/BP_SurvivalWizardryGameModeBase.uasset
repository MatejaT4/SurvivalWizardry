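; Game mode Blueprint for Survival Wizardry that drives the UI at each stage of a match.
; Separate events create the countdown widget, the in-game progress, time and current spells widgets, and the win or death end screen.
; Game start and end also call spawn dispatchers to signal spawning.
; Level-up pauses the game and shows the level-up widget, with no unpause in this graph.
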(event `self.StartGameCountdownEvent`
  (bind _returnvalue (`|CreateWidget` "/Game/Widgets/StartWidget.StartWidget_C"))
  (set `/Game/Widgets/StartWidget.CountDown` (`KismetMathLibrary.Conv_IntToDouble` (`self.GameCountdownLength`)) _returnvalue)
  (`UserWidget.AddToViewport` _returnvalue 0))

(event `self.StartGameEvent`
  (bind _returnvalue (`|CreateWidget` "/Game/Widgets/ProgressWidget.ProgressWidget_C"))
  (`UserWidget.AddToViewport` _returnvalue 0)
  (bind _returnvalue_2 (`|CreateWidget` "/Game/Widgets/TimeWidget.TimeWidget_C"))
  (`UserWidget.AddToViewport` _returnvalue_2 0)
  (bind _returnvalue_3 (`|CreateWidget` "/Game/Widgets/CurrentSpellsWidget.CurrentSpellsWidget_C"))
  (`UserWidget.AddToViewport` _returnvalue_3 0)
  (`self.StartSpawnDispatcher`))

(event `self.EndGameEvent`
  (params (bGameWon :type Boolean))
  (bind _returnvalue (`|CreateWidget` "/Game/Widgets/EndWidget.EndWidget_C"))
  (`UserWidget.AddToViewport` _returnvalue 0)
  (`TextBlock.SetText` (`/Game/Widgets/EndWidget.ResultText` _returnvalue) (select `bool` bGameWon :`false` "You    Died" :`true` "You    Won" :!type "Text"))
  (`self.EndSpawnDispecher`))

(event `self.LevelUpEvent`
  (`GameplayStatics.SetGamePaused` true)
  (bind _returnvalue (`|CreateWidget` "/Game/Widgets/LevelUpWidget.LevelUpWidget_C"))
  (`UserWidget.AddToViewport` _returnvalue 0))

(fn `UserConstructionScript`)