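; BP_Spawner spawns enemies and health packs in the Survival Wizardry game.
; On BeginPlay it binds its start and stop events to dispatchers on the game mode.
; Starting sets a looping health pack timer and a one-shot Cubie timer, then plays a timeline whose event tracks spawn Cubie, Ballzie, Chunker and Signor Diamante enemies at per-type heights.
; Stopping halts the timeline but leaves the timers uncleared.
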(event `self.ReceiveBeginPlay`
  (bind _returnvalue (`GameplayStatics.GetActorOfClass` "/Game/Blueprints/BP_SurvivalWizardryGameModeBase.BP_SurvivalWizardryGameModeBase_C"))
  (add `/Game/Blueprints/BP_SurvivalWizardryGameModeBase.SpawnDispatcher` _returnvalue (delegate `SpawnerBegin`))
  (add `/Game/Blueprints/BP_SurvivalWizardryGameModeBase.EndSpawnDispecher` _returnvalue (delegate `Stop Spawning`)))

(event `Stop Spawning`
  (`Timeline|Timeline_0` :!via `Stop` :!label _label
    (:`Cubie`
      (`self.SpawnEnemy` "/Game/Blueprints/Enemies/BP_Cubie.BP_Cubie_C" 90.0))
    (:`Ballzie`
      (`self.SpawnEnemy` "/Game/Blueprints/Enemies/BP_Ballzie.BP_Ballzie_C" 60.0))
    (:`Chunker`
      (`self.SpawnEnemy` "/Game/Blueprints/Enemies/BP_Chunker.BP_Chunker_C" 150.0))
    (:`SignorDiamante`
      (`self.SpawnEnemy` "/Game/Blueprints/Enemies/BP_SignorDiamante.BP_SignorDiamante_C" 120.0))))

(event `SpawnerBegin`
  (`KismetSystemLibrary.K2_SetTimerDelegate` (delegate `spawn health pack`) 2.0 true)
  (`KismetSystemLibrary.K2_SetTimerDelegate` (delegate `spawn cubie`) 1.5)
  (goto _label :!via `PlayFromStart`))

(event `spawn cubie`
  (`self.SpawnEnemy` "/Game/Blueprints/Enemies/BP_Cubie.BP_Cubie_C" 90.0))

(event `spawn health pack`
  (`self.SpawnHealtHPack` "/Game/Blueprints/BP_HealthPack.BP_HealthPack_C" 90.0))

(fn `UserConstructionScript`)