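; BP_Cubie is an enemy Blueprint that animates the scale of its CollisionMesh when play begins.
; Timeline_1 drives the scale first, then hands off to Timeline_0 when it finishes.
; Each update converts the track value to a vector and sets the world transform, keeping location and rotation unchanged.
; The construction script only calls its parent, and no other gameplay logic is active here.
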(event `self.ReceiveBeginPlay`
  (bind _collisionmesh (`self.CollisionMesh`))
  (bind _collisionmesh_2 (`self.CollisionMesh`))
  (bind (_returnvalue_location _returnvalue_rotation) (`KismetMathLibrary.BreakTransform` (`SceneComponent.K2_GetComponentToWorld` _collisionmesh_2)))
  (bind (_returnvalue_location_2 _returnvalue_rotation_2) (`KismetMathLibrary.BreakTransform` (`SceneComponent.K2_GetComponentToWorld` _collisionmesh)))
  (bind (_direction _newtrack_0) (`Timeline|Timeline_1` :!via `PlayFromStart`)
    (:`Update`
      (`SceneComponent.K2_SetWorldTransform` _collisionmesh_2 (`KismetMathLibrary.MakeTransform` _returnvalue_location _returnvalue_rotation (`KismetMathLibrary.Conv_DoubleToVector` _newtrack_0)) false false))
    (:`Finished`
      (bind (_direction_2 _newtrack_0_2) (`Timeline|Timeline_0` :!via `PlayFromStart`)
        (:`Update`
          (`SceneComponent.K2_SetWorldTransform` _collisionmesh (`KismetMathLibrary.MakeTransform` _returnvalue_location_2 _returnvalue_rotation_2 (`KismetMathLibrary.Conv_DoubleToVector` _newtrack_0_2)) false false))))))

(fn `UserConstructionScript`
  (`parent.UserConstructionScript`))