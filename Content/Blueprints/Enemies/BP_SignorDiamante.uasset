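; BP_SignorDiamante is an enemy Blueprint that periodically telegraphs and performs a short speed burst.
; A looping five-second timer fires Whooosh, which plays a timeline that animates the Base Color material parameter on two static meshes.
; When the timeline finishes, Speed jumps for one second, then drops back to a slower value.
; The graph only sets Speed and contains no movement logic of its own.
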(event `self.ReceiveBeginPlay`
  (`KismetSystemLibrary.K2_SetTimerDelegate` (delegate `Whooosh`) 5.0 true))

(event `Whooosh`
  (bind (_direction _newtrack_1) (`Timeline|Timeline_0` :!via `PlayFromStart`)
    (:`Update`
      (bind _returnvalue (`KismetMathLibrary.Conv_LinearColorToVector` _newtrack_1))
      (`MeshComponent.SetVectorParameterValueOnMaterials` (`self.StaticMesh2`) "Base Color" _returnvalue)
      (`MeshComponent.SetVectorParameterValueOnMaterials` (`self.StaticMesh1`) "Base Color" _returnvalue))
    (:`Finished`
      (set `self.Speed` 800.0)
      (`KismetSystemLibrary.Delay` 1.0)
      (set `self.Speed` 200.0))))

(fn `UserConstructionScript`
  (`parent.UserConstructionScript`))